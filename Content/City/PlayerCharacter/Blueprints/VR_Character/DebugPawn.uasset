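; DebugPawn is a debug pawn for placing road, commercial and residential city tiles on a grid.
; Number keys spawn the held tile, which follows an eye-view line trace snapped to 100-unit cells at ground height.
; Left click rejects occupied cells in red or commits the tile, setting its material or linking new roads with existing ones.
; Right click destroys the held tile, and P calls SpawnMoney on the GS_MainMenu game state.
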(event `Key|Three`
  (params (Key :type "Key Structure"))
  (:`Pressed`
    (`self.K2_DestroyActor` (`self.Selected Tile`))
    (bind _returnvalue (`|SpawnActorFromClass` "/Game/LevelContent/Meshes/Residential/Residential.Residential_C" (`self.FloorTransform`) "Undefined" "OverrideRootScale" null null))
    (set `self.Selected Tile` _returnvalue)))

(event `Key|Two`
  (params (Key :type "Key Structure"))
  (:`Pressed`
    (`self.K2_DestroyActor` (`self.Selected Tile`))
    (bind _returnvalue (`|SpawnActorFromClass` "/Game/LevelContent/Meshes/Commercial/Commercial.Commercial_C" (`self.FloorTransform`) "Undefined" "OverrideRootScale" null null))
    (set `self.Selected Tile` _returnvalue)))

(event `Key|One`
  (params (Key :type "Key Structure"))
  (:`Pressed`
    (`self.K2_DestroyActor` (`self.Selected Tile`))
    (bind _returnvalue (`|SpawnActorFromClass` "/Game/LevelContent/Meshes/Road/Road.Road_C" (`self.FloorTransform`) "Undefined" "OverrideRootScale" null null))
    (set `self.Selected Tile` _returnvalue)))

(event `self.ReceiveTick`
  (params (DeltaSeconds :type "Float (single-precision)"))
  (bind _floor_location (`self.Floor Location`))
  (set `self.FloorTransform` (`KismetMathLibrary.Conv_VectorToTransform` _floor_location))
  (if (!= (`self.Selected Tile`) null)
    (`self.K2_SetActorLocation` (`self.Selected Tile`) _floor_location false false)))

(event `Key|RightMouseButton`
  (params (Key :type "Key Structure"))
  (:`Pressed`
    (if (!= (`self.Selected Tile`) null)
      (`self.K2_DestroyActor` (`self.Selected Tile`)))))

(event `Key|LeftMouseButton`
  (params (Key :type "Key Structure"))
  (:`Pressed`
    (if (!= (`self.Selected Tile`) null)
      (bind _allowed (`self.Validate Tile` (`self.Tiles`) (`self.Selected Tile`)))
      (if _allowed
        (`KismetArrayLibrary.Array_Add` (`self.Tiles`) (`self.Selected Tile`))
        (set `self.Selected Tile` null)))))

(event `Key|P`
  (params (Key :type "Key Structure"))
  (:`Pressed`
    (bind _asgs_main_menu (cast `/Game/Maps/GS_MainMenu` (`GameplayStatics.GetGameState`)))
    (`/Game/Maps/GS_MainMenu.SpawnMoney` _asgs_main_menu)))

(fn `Floor Location`
  (returns (`Floor Location` :type "Vector Structure"))
  (bind (_outlocation _outrotation) (`self.GetActorEyesViewPoint`))
  (bind _100 (`self.100`))
  (bind _outhit (`KismetSystemLibrary.LineTraceSingle` _outlocation (+ _outlocation (* (`KismetMathLibrary.GetForwardVector` _outrotation) 50000)) "TraceTypeQuery1"))
  (bind (_returnvalue_x _returnvalue_y) (`KismetMathLibrary.BreakVector` (* (`.ImpactPoint` (`GameplayStatics.BreakHitResult` _outhit)) (1.0 1.0 0.0))))
  (return (`KismetMathLibrary.MakeVector` (* (`KismetMathLibrary.Round` (/ _returnvalue_x _100)) _100) (* (`KismetMathLibrary.Round` (/ _returnvalue_y _100)) _100))))

(fn `Road Manager`
  (params (`New Tile` :type "Actor Object Reference"))
  (locals (`Road Connections` :type Integer) (Index :type Integer) (`New Road` :type String))
  (bind _roads (`self.Roads`))
  (bind _asroad (cast `/Game/LevelContent/Meshes/Road/Road` `New Tile`)
    (:`then`
      (for _array_element _roads
        (bind _asroad_2 (cast `/Game/LevelContent/Meshes/Road/Road` _array_element))
        (`/Game/LevelContent/Meshes/Road/Road.ValidateRoadsEvent` _asroad_2 _asroad))
      (`KismetArrayLibrary.Array_Add` _roads _asroad)
      (`/Game/LevelContent/Meshes/Road/Road.AddRoad` _asroad))
    (:`CastFailed`
      _))
  (return))

(fn `SetMaterial`
  (params (`New Tile` :type "Actor Object Reference"))
  (locals (TempNewTile :type "SceneComponent Object Reference"))
  (bind _returnvalue (`SceneComponent.GetChildComponent` (`self.K2_GetRootComponent` `New Tile`) 0))
  (if (`self.ActorHasTag` `New Tile` "Commercial")
    (bind _asprimitive_component (cast `PrimitiveComponent` _returnvalue)
      (:`then`
        _)
      (:`CastFailed`
        _))
    (`PrimitiveComponent.SetMaterial` _asprimitive_component 0 "/Game/LevelContent/Material.Material")
    (elif (`self.ActorHasTag` `New Tile` "Road")
      (`self.Road Manager` `New Tile`)
      (elif (`self.ActorHasTag` `New Tile` "Residential")
        (bind _asprimitive_component_2 (cast `PrimitiveComponent` _returnvalue)
          (:`then`
            _)
          (:`CastFailed`
            _))
        (`PrimitiveComponent.SetMaterial` _asprimitive_component_2 0 "/Game/LevelContent/Material.Material")
        (else
          (`KismetSystemLibrary.PrintString` "Tags not working")))))
  (return))

(fn `UserConstructionScript`)

(fn `Validate Tile`
  (params (`Tile Array` :type "Array of Actor Object Reference") (`New Tile` :type "Actor Object Reference"))
  (returns (Allowed :type Boolean))
  (locals (IsAllowed :type Boolean))
  (bind _returnvalue (`self.K2_GetRootComponent` `New Tile`))
  (set `local.IsAllowed` true)
  (for _array_element `Tile Array`
    (if (== (`SceneComponent.K2_GetComponentLocation` _returnvalue) (`SceneComponent.K2_GetComponentLocation` (`self.K2_GetRootComponent` _array_element)))
      (bind _asprimitive_component (cast `PrimitiveComponent` (`SceneComponent.GetChildComponent` _returnvalue 0))
        (:`then`
          (`PrimitiveComponent.SetMaterial` _asprimitive_component 0 "/Game/PlayerCharacter/Blueprints/VR_Character/REd.REd"))
        (:`CastFailed`
          _))
      (set `local.IsAllowed` false)
      (return (`local.IsAllowed`))))
  (`self.SetMaterial` `New Tile`)
  (return (`local.IsAllowed`)))