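; Planet actor that sizes its sphere mesh from a radius in meters and populates its surface with resources and colonies.
; On BeginPlay it caches the Sun, then spawns each listed class at its origin with random rotation, pushed out along local Z by radius plus offset.
; Colonies receive the radius and update their rings.
; A helper projects locations onto the surface with normals; the orbit/spin logic is disconnected.
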(event `self.ReceiveBeginPlay`
  (bind _outactors (`GameplayStatics.GetAllActorsOfClass` "/Game/Planet/Sun.Sun_C"))
  (bind _assun (cast `/Game/Planet/Sun` (`|GetArrayItem` _outactors)))
  (set `self.Orbiting` _assun)
  (`self.SpawnRes`)
  (`self.SpawnColony`))

(event `self.ReceiveTick`
  (params (DeltaSeconds :type "Float (single-precision)")))

(fn `GetSurfaceLocationAndNormalAt`
  (params (Location :type "Vector Structure"))
  (returns (SurfaceLocation :type "Vector Structure") (SurfaceNormal :type "Vector Structure"))
  (bind _returnvalue (`KismetMathLibrary.Normal` (- Location (`self.K2_GetActorLocation`))))
  (return (+ (* _returnvalue (`self.RadiusInUnits`)) (`self.K2_GetActorLocation`)) _returnvalue))

(fn `SpawnColony`
  ;[1 1 1] Установка городов на планете
  (for _array_element (`self.ArrayColony`)
    (bind _returnvalue (`|SpawnActorFromClass` _array_element (`KismetMathLibrary.MakeTransform` (`self.K2_GetActorLocation`) (`KismetMathLibrary.RandomRotator` false) (-0.6 -0.6 0.9)) "Undefined" "OverrideRootScale" self null))
    (`self.K2_AddActorLocalOffset` _returnvalue (`KismetMathLibrary.MakeVector` 0.0 0.0 (+ (+ (.z (`self.K2_GetActorLocation`)) (`self.RadiusInUnits`)) 3335.0)) false false)
    (bind _asspace_colony_bp (cast `/Game/Blueprints/SpaceColony_BP` _returnvalue))
    (set `/Game/Blueprints/SpaceColony_BP.RadiusPlanet` (`self.RadiusInUnits`) _asspace_colony_bp)
    (`/Game/Blueprints/SpaceColony_BP.ChangeRings` _asspace_colony_bp)))

(fn `SpawnRes`
  (for _array_element (`self.ArrayResurce`)
    (bind _returnvalue (`|SpawnActorFromClass` _array_element (`KismetMathLibrary.MakeTransform` (`self.K2_GetActorLocation`) (`KismetMathLibrary.RandomRotator` true)) "Undefined" "OverrideRootScale" self null))
    (`self.K2_AddActorLocalOffset` _returnvalue (`KismetMathLibrary.MakeVector` 0.0 0.0 (+ (+ (.z (`self.K2_GetActorLocation`)) (`self.RadiusInUnits`)) 3200.0)) false false)))

(fn `UserConstructionScript`
  (bind _output_get (set `self.RadiusInUnits` (* (`self.RadiusInMeters`) 100.0)))
  (`SceneComponent.SetWorldScale3D` (`self.Planet`) (`KismetMathLibrary.Conv_DoubleToVector` (/ _output_get (.x (`.BoxExtent` (`KismetSystemLibrary.GetComponentBounds` (`self.Planet`)))))))
  (`SceneComponent.K2_SetRelativeLocation` (`self.Planet`) (`KismetMathLibrary.MakeVector` 0.0 0.0 (- 0.0 _output_get)) false false))