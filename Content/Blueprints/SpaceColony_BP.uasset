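; SpaceColony_BP is a space colony (city) actor that shows its level as a stack of rings.
; The ChangeRings event loops up to ColonyLevel, spawning RingColony_BP actors at the colony's position and rotation, each higher, wider and flatter.
; CurrentRenderLevelColony skips spawning once it matches the level, but a level increase respawns from the first ring without removing existing ones.
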(event `ChangeRings`
  (bind (_returnvalue_roll _returnvalue_pitch _returnvalue_yaw) (`KismetMathLibrary.BreakRotator` (`self.K2_GetActorRotation`)))
  (bind (_returnvalue_x _returnvalue_y _returnvalue_z) (`KismetMathLibrary.BreakVector` (`self.K2_GetActorLocation`)))
  ;[1 1 1] Добавляем кольца для городу
  (for _index (range 1 (+ (`self.ColonyLevel`) 1))
    (if (not (== (`self.CurrentRenderLevelColony`) (`self.ColonyLevel`)))
      (bind _returnvalue (`KismetMathLibrary.Conv_IntToDouble` _index))
      (`|SpawnActorFromClass` "/Game/Blueprints/RingColony_BP.RingColony_BP_C" (`KismetMathLibrary.MakeTransform` (`KismetMathLibrary.MakeVector` _returnvalue_x _returnvalue_y (+ _returnvalue_z _returnvalue)) (`KismetMathLibrary.MakeRotator` _returnvalue_roll _returnvalue_pitch _returnvalue_yaw) (`KismetMathLibrary.MakeVector` (+ _returnvalue 0.6) (+ _returnvalue 0.6) (- 0.9 (/ _returnvalue 10.0)))) "Undefined" "OverrideRootScale" null null)
      (set `self.CurrentRenderLevelColony` _index))))

(event `self.ReceiveBeginPlay`)

(fn `UserConstructionScript`)